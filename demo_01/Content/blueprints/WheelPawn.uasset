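; Player-controlled wheel pawn that rolls and steers as a Newton Dynamics rigid body.
; Axis inputs store drive and turn values, which the Newton force-and-torque callback turns into torque.
; Drive torque acts about the body's right axis with damping on that spin, while steering torque acts about the horizontal forward axis to turn by leaning.
; The callback also adds a mass-scaled acceleration force.
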(event Custom|OnNewtonForceAndTorque
  (bind _newtonrigidbody (Variables|Default|GetNewtonRigidBody))
  (bind _returnvalue (Class|NewtonRigidBody|GetRightDir _newtonrigidbody))
  (Class|NewtonRigidBody|SetForce (Variables|Default|GetNewtonRigidBody) (+ (* (Class|NewtonRigidBody|GetMass (Variables|Default|GetNewtonRigidBody)) (Variables|Default|Getacceleration)) (Class|NewtonRigidBody|GetForce (Variables|Default|GetNewtonRigidBody))))
  (Class|NewtonRigidBody|SetTorque (Variables|Default|GetNewtonRigidBody) (+ (* (- (* (Variables|Default|GetForwardKey) (Variables|Default|GetForwardTorque)) (* (Math|Vector|DotProduct (Class|NewtonRigidBody|GetOmega (Variables|Default|GetNewtonRigidBody)) _returnvalue) (Variables|Default|GetlongitudinalDamp))) _returnvalue) (* (Math|Vector|CrossProduct (Variables|Default|GetUpDir) (Class|NewtonRigidBody|GetRightDir (Variables|Default|GetNewtonRigidBody))) (* (Variables|Default|GetTurnKey) (Variables|Default|GetTurnTorque))))))

(event Input|AxisEvents|InputAxisForwardBack
  (params (AxisValue :type Float%20%28single-precision%29))
  ;[1 1 1] Get Input Events
  (Variables|Default|SetForwardKey AxisValue))

(event Input|AxisEvents|InputAxisTurnLeftRight
  (params (AxisValue :type Float%20%28single-precision%29))
  ;[1 1 1] Get Input Events
  (Variables|Default|SetTurnKey AxisValue))

(fn ConstructionScript)