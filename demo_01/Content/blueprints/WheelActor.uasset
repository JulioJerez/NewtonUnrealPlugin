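; WheelActor is a physics wheel driven through a Newton rigid body's force-and-torque callback, apparently an early test.
; Each callback adds mass times Acceleration to the body's force, noted as anti-gravity.
; It sets torque along the right axis: drive Torque is multiplied by zero, leaving quadratic spin damping signed by Torque.
; The ForwardBack axis only prints a debug string.
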(event Custom|OnNewtonForceAndTorque
  (params (timesteo :type Float%20%28double-precision%29))
  (bind _newtonrigidbody (Variables|Default|GetNewtonRigidBody))
  (bind _newtonrigidbody_2 (Variables|Default|GetNewtonRigidBody))
  (bind _returnvalue (Class|NewtonRigidBody|GetOmega _newtonrigidbody))
  (bind _returnvalue_2 (Class|NewtonRigidBody|GetRightDir _newtonrigidbody_2))
  (bind _returnvalue_3 (Math|Vector|DotProduct _returnvalue _returnvalue_2))
  (Class|NewtonRigidBody|SetForce (Variables|Default|GetNewtonRigidBody) (+ (* (Class|NewtonRigidBody|GetMass (Variables|Default|GetNewtonRigidBody)) (Variables|Default|Getacceleration)) (Class|NewtonRigidBody|GetForce (Variables|Default|GetNewtonRigidBody))))
  (Class|NewtonRigidBody|SetTorque (Variables|Default|GetNewtonRigidBody) (* (- (* 0.0 (Variables|Default|GetTorque)) (* (* _returnvalue_3 _returnvalue_3) (* (Variables|Default|GetlongitudinalDamp) (Math|Float|Sign(Float) (Variables|Default|GetTorque))))) (Class|NewtonRigidBody|GetRightDir (Variables|Default|GetNewtonRigidBody)))))

(event Input|AxisEvents|InputAxisForwardBack
  (params (AxisValue :type Float%20%28single-precision%29))
  (Development|PrintString "Hello"))

(fn ConstructionScript)